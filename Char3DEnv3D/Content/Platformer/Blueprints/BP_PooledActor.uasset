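; BP_PooledActor is an actor meant for object pooling, switched between in-use and idle states instead of being spawned and destroyed.
; SetInUse toggles collision, visibility and tick together, and the actor starts idle on BeginPlay.
; Activation starts a TimeToLive timer that calls ReturnToPool to deactivate it, and each state change clears any pending timer first.
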(event Custom|SetInUse
  (params (IsInUse :type Boolean))
  (Variables|Default|SetIsInUse IsInUse)
  (Collision|SetActorEnableCollision IsInUse)
  (Rendering|SetActorHiddenInGame (not IsInUse))
  (Actor|Tick|SetActorTickEnabled IsInUse)
  (Utilities|Time|ClearandInvalidateTimerbyHandle (Variables|Default|GetTimeToLiveTimer))
  (if IsInUse
    (bind _returnvalue (Utilities|Time|SetTimerbyEvent (delegate Custom|ReturnToPool) (Variables|Default|GetTimeToLive)))
    (Variables|Default|SetTimeToLiveTimer _returnvalue)))

(event Custom|ReturnToPool
  (CallFunction|SetinUse false))

(event EventBeginPlay
  (CallFunction|SetinUse false))

(fn ConstructionScript)