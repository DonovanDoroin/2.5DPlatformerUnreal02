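; Goomba-style Paper2D platformer enemy that damages the player on overlap and awards points when stomped or hit by a pooled fireball.
; A Tick gate, opened by PlayerDetectRange, drives either seeking the player or pacing that reverses on wall hits.
; A downward hit normal on StompBox triggers a squish and delayed explosion, while fireballs destroy it immediately.
; Construction derives walk speed and flipbook play rate from Speed.
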(event OnComponentBeginOverlap(Collider)
  (params (OverlappedComponent :type Primitive%20Component%20Object%20Reference) (OtherActor :type Actor%20Object%20Reference) (OtherComp :type Primitive%20Component%20Object%20Reference) (OtherBodyIndex :type Integer) (bFromSweep :type Boolean) (SweepResult :type Hit%20Result%20Structure%20%28by%20ref%29))
  ;[1 1 1] Goomba Damages Player
  (bind _asbp_third_person_character (Utilities|Casting|CastToBP_ThirdPersonCharacter OtherActor))
  (Default|AdjustHitPoints _asbp_third_person_character (Variables|Default|GetHealthToSubtract)))

(event OnComponentHit(StompBox)
  (params (HitComponent :type Primitive%20Component%20Object%20Reference) (OtherActor :type Actor%20Object%20Reference) (OtherComp :type Primitive%20Component%20Object%20Reference) (NormalImpulse :type Vector :default "0, 0, 0") (Hit :type Hit%20Result%20Structure%20%28by%20ref%29))
  (bind _paperflipbook (Variables|Default|GetPaperFlipbook))
  (if (and (== OtherActor (Game|GetPlayerCharacter 0)) (Utilities|Operators|EqualEqual (.ImpactNormal (Collision|BreakHitResult Hit)) "0.000000,0.000000,-1.000000" 0.1))
    (Utilities|FlowControl|Sequence
      (:then_0
        ;[1 1 1] Enemy Squish Effects
        (Audio|PlaySound2D "/Game/Platformer/Audio/Mario_Squish.Mario_Squish" 1.0 1.0 0.0 0 0)
        (Collision|SetCollisionEnabled (Variables|Default|GetCollider) "NoCollision")
        (Components|DestroyComponent (Variables|Default|GetStompBox))
        (Transformation|SetWorldScale3D _paperflipbook "0.250000,0.250000,0.100000")
        (Transformation|AddWorldOffset _paperflipbook "0.000000,0.000000,-35.000000" false false)
        (Pawn|Components|CharacterMovement|DisableMovement (Variables|Character|GetCharacterMovement)))
      (:then_1
        ;[1 1 1] Show Add Points
        (Game|SpawnActorfromClass "/Game/Platformer/Blueprints/BP_Points.BP_Points_C" (Transformation|GetActorTransform) "Undefined" "MultiplyWithRoot" 0 (Variables|Default|GetPoints) 0)
        (Default|AddPoints (Variables|Default|GetAs%20BP%20Player%20Controller) (Variables|Default|GetPoints)))
      (:then_2
        ;[1 1 1] Play Destroy FX
        (Utilities|FlowControl|Delay 0.5)
        (CallFunction|PlayBlockInteractEffect "/Game/StarterContent/Audio/Explosion_Cue.Explosion_Cue" 0 "/Game/InfinityBladeEffects/Effects/FX_Monsters/FX_Monster_Gruntling/FlameThrower/P_FlameExplode.P_FlameExplode" (Transformation|GetWorldLocation (Variables|Default|GetCollider)))
        (Actor|DestroyActor)))))

(event OnComponentHit(Collider)
  (params (HitComponent :type Primitive%20Component%20Object%20Reference) (OtherActor :type Actor%20Object%20Reference) (OtherComp :type Primitive%20Component%20Object%20Reference) (NormalImpulse :type Vector :default "0, 0, 0") (Hit :type Hit%20Result%20Structure%20%28by%20ref%29))
  (bind _asbp_fireball (Utilities|Casting|CastToBP_Fireball OtherActor))
  (Default|ReturntoPool _asbp_fireball)
  (Utilities|FlowControl|Sequence
    (:then_0
      ;[1 1 1] Show Add Points
      (Game|SpawnActorfromClass "/Game/Platformer/Blueprints/BP_Points.BP_Points_C" (Transformation|GetActorTransform) "Undefined" "MultiplyWithRoot" 0 (Variables|Default|GetPoints) 0)
      (Default|AddPoints (Variables|Default|GetAs%20BP%20Player%20Controller) (Variables|Default|GetPoints)))
    (:then_1
      ;[1 1 1] Play Destroy FX
      (CallFunction|PlayBlockInteractEffect "/Game/StarterContent/Audio/Explosion_Cue.Explosion_Cue" 0 "/Game/InfinityBladeEffects/Effects/FX_Monsters/FX_Monster_Gruntling/FlameThrower/P_FlameExplode.P_FlameExplode" (Transformation|GetWorldLocation (Variables|Default|GetCollider)))
      (Actor|DestroyActor))))

(event OnComponentBeginOverlap(PlayerDetectRange)
  (params (OverlappedComponent :type Primitive%20Component%20Object%20Reference) (OtherActor :type Actor%20Object%20Reference) (OtherComp :type Primitive%20Component%20Object%20Reference) (OtherBodyIndex :type Integer) (bFromSweep :type Boolean) (SweepResult :type Hit%20Result%20Structure%20%28by%20ref%29))
  (bind _returnvalue (Game|GetPlayerCharacter 0))
  (bind _paperflipbook (Variables|Default|GetPaperFlipbook))
  (bind _paperflipbook_2 (Variables|Default|GetPaperFlipbook))
  (bind _returnvalue_2 (Transformation|GetWorldScale _paperflipbook))
  (bind _returnvalue_3 (Transformation|GetWorldScale _paperflipbook_2))
  ;[1 1 1] Move Goomba in Given Direction only IF player is in Range
  (if (== OtherActor (Game|GetPlayerCharacter 0))
    (Utilities|FlowControl|Gate true) ; enters at Open
  ))

(event OnComponentEndOverlap(CapsuleComponent)
  (params (OverlappedComponent :type Primitive%20Component%20Object%20Reference) (OtherActor :type Actor%20Object%20Reference) (OtherComp :type Primitive%20Component%20Object%20Reference) (OtherBodyIndex :type Integer))
  (bind _returnvalue (Game|GetPlayerCharacter 0))
  (bind _paperflipbook (Variables|Default|GetPaperFlipbook))
  (bind _paperflipbook_2 (Variables|Default|GetPaperFlipbook))
  (bind _returnvalue_2 (Transformation|GetWorldScale _paperflipbook))
  (bind _returnvalue_3 (Transformation|GetWorldScale _paperflipbook_2))
  ;[1 1 1] Move Goomba in Given Direction only IF player is in Range
  (if (== (Game|GetPlayerCharacter 0) OtherActor)
    (Utilities|FlowControl|Gate true) ; enters at Close
  ))

(event OnComponentHit(CapsuleComponent)
  (params (HitComponent :type Primitive%20Component%20Object%20Reference) (OtherActor :type Actor%20Object%20Reference) (OtherComp :type Primitive%20Component%20Object%20Reference) (NormalImpulse :type Vector :default "0, 0, 0") (Hit :type Hit%20Result%20Structure%20%28by%20ref%29))
  (Utilities|FlowControl|DoOnce false :!label _label
    (:Completed
      (if (Utilities|Operators|EqualEqual (Math|Vector|VectorGetAbs (.ImpactNormal (Collision|BreakHitResult Hit))) "1.000000,0.000000,0.000000" 0.1)
        (Utilities|FlowControl|FlipFlop
          (:A
            (Variables|Default|SetIsMoveLeft false))
          (:B
            (Variables|Default|SetIsMoveLeft true)))
        (Utilities|FlowControl|Delay 0.5)
        (goto _label Reset)))))

(event EventBeginPlay
  ;[1 1 1] Reference to Player Controller
  (bind _asbp_player_controller (Utilities|Casting|CastToBP_PlayerController (Game|GetPlayerController 0)))
  (Variables|Default|SetAs%20BP%20Player%20Controller _asbp_player_controller))

(event EventTick
  (params (DeltaSeconds :type Float%20%28single-precision%29))
  (bind _returnvalue (Game|GetPlayerCharacter 0))
  (bind _paperflipbook (Variables|Default|GetPaperFlipbook))
  (bind _paperflipbook_2 (Variables|Default|GetPaperFlipbook))
  (bind _returnvalue_2 (Transformation|GetWorldScale _paperflipbook))
  (bind _returnvalue_3 (Transformation|GetWorldScale _paperflipbook_2))
  ;[1 1 1] Move Goomba in Given Direction only IF player is in Range
  (Utilities|FlowControl|Gate true
    (:Exit
      (if (Variables|Default|GetIsSeekerEnemny)
        (AI|Navigation|SimpleMovetoActor (Pawn|GetController) _returnvalue)
        (if (< (.x (Transformation|GetActorLocation _returnvalue)) (.x (Transformation|GetActorLocation)))
          (Transformation|SetWorldScale3D _paperflipbook (Math|Vector|MakeVector (Math|Float|Absolute(Float) (.x _returnvalue_2)) (.y _returnvalue_2) (.z _returnvalue_2)))
          (else
            (Transformation|SetWorldScale3D _paperflipbook_2 (Math|Vector|MakeVector (* (Math|Float|Absolute(Float) (.x _returnvalue_3)) -1.0) (.y _returnvalue_3) (.z _returnvalue_3)))))
        (else
          (Pawn|Input|AddMovementInput (Math|Vector|SelectVector "1.000000,0.000000,0.000000" "-1.000000,0.000000,0.000000" (Variables|Default|GetIsMoveLeft)) 1.0 false)
          (Components|Timeline|SetPlayRate (Variables|Default|GetPaperFlipbook) (Variables|Default|GetFlipbookRateMultiplier)))))))

(fn ConstructionScript
  (bind _output_get (Variables|/Script/Engine.CharacterMovementComponent|SetMaxWalkSpeed (Variables|Character|GetCharacterMovement) (Variables|Default|GetSpeed)))
  (Variables|Default|SetFlipbookRateMultiplier (Math|Float|Clamp(Float) (/ _output_get 1e+02) 0.1 3.0)))