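; Base platformer block that reacts to player hits and can turn into a collectible coin during a P-Block effect.
; A player hit on the cube with an impact normal Z of exactly 1 calls HitBlockMessage.
; PBlockOn hides the cube, disables its collision and shows the child actor, while PBlockOff reverses this.
; Player overlap with CoinCollider destroys the block, and BeginPlay caches the player controller.
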(event OnComponentHit(Cube)
  (params (HitComponent :type Primitive%20Component%20Object%20Reference) (OtherActor :type Actor%20Object%20Reference) (OtherComp :type Primitive%20Component%20Object%20Reference) (NormalImpulse :type Vector :default "0, 0, 0") (Hit :type Hit%20Result%20Structure%20%28by%20ref%29))
  (if (and (== OtherActor (Game|GetPlayerCharacter 0)) (== (.Z (Math|Vector|BreakVector (.ImpactNormal (Collision|BreakHitResult Hit)))) 1.0))
    (Class|BPIPlatform|HitBlock(Message) self)))

(event OnComponentBeginOverlap(CoinCollider)
  (params (OverlappedComponent :type Primitive%20Component%20Object%20Reference) (OtherActor :type Actor%20Object%20Reference) (OtherComp :type Primitive%20Component%20Object%20Reference) (OtherBodyIndex :type Integer) (bFromSweep :type Boolean) (SweepResult :type Hit%20Result%20Structure%20%28by%20ref%29))
  ;[1 1 1] Destrpy Block if PBlock coin inside is collected
  (if (== OtherActor (Game|GetPlayerCharacter 0))
    (Actor|DestroyActor)))

(event EventBeginPlay
  ;[1 1 1] Ref to Player Controller
  (bind _asbp_player_controller (Utilities|Casting|CastToBP_PlayerController (Game|GetPlayerController 0)))
  (Variables|Default|SetAsBPPlayerController _asbp_player_controller))

(fn ConstructionScript)

(fn PBlockon
  (bind _cube (Variables|Default|GetCube))
  (Rendering|SetVisibility _cube false false)
  (Collision|SetCollisionEnabled _cube "NoCollision")
  (Rendering|SetVisibility (Variables|Default|GetChildActor) true false))

(fn PBlockOff
  (bind _cube (Variables|Default|GetCube))
  (Rendering|SetVisibility _cube true false)
  (Collision|SetCollisionEnabled _cube "QueryAndPhysics")
  (Rendering|SetVisibility (Variables|Default|GetChildActor) false false))