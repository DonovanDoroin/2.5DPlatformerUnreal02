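; A Mario-style P-Block that, when the player stomps it, temporarily switches on all tagged blocks.
; A downward-normal hit bounces the character, plays smash effects and feedback, swaps to smashed meshes and replaces level music with its own.
; It calls PBlockOn on tagged BP_Block_Base actors and starts a timer.
; Timer expiry, player death or level completion calls PBlockOff and restores the level music.
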(event OnComponentHit(Box)
  (params (HitComponent :type Primitive%20Component%20Object%20Reference) (OtherActor :type Actor%20Object%20Reference) (OtherComp :type Primitive%20Component%20Object%20Reference) (NormalImpulse :type Vector :default "0, 0, 0") (Hit :type Hit%20Result%20Structure%20%28by%20ref%29))
  (bind _asbp_third_person_character (Utilities|Casting|CastToBP_ThirdPersonCharacter OtherActor))
  (if (Utilities|Operators|EqualEqual (.ImpactNormal (Collision|BreakHitResult Hit)) "0.000000,0.000000,-1.000000" 0.01)
    (Character|LaunchCharacter _asbp_third_person_character "0.000000,0.000000,400.000000" false false)
    (Utilities|FlowControl|Sequence
      (:then_0
        ;[1 1 1] PBlock FX
        (Audio|PlaySound2D "/Game/Platformer/Audio/Mario_Thwomp.Mario_Thwomp" 1.0 1.0 0.0 0 0)
        (Effects|SpawnEmitteratLocation "/Game/InfinityBladeEffects/Effects/FX_Breakables/pot/P_PotBreak_Ceramic.P_PotBreak_Ceramic" (Transformation|GetWorldLocation (Variables|Default|GetBlock_P_Base_Smashed)))
        (Audio|Components|Audio|Play (Variables|Default|GetMusic) 0.0)
        ;[1 1 1] Pause Level Music
        (Class|AudioComponent|SetPaused (Variables|/Game/Platformer/Blueprints/BP_LevelSettings.BP_LevelSettings_C|GetLevelMusic (Variables|Default|GetLevelSettings)) true))
      (:then_1
        ;[1 1 1] Camera shake and force feedback
        (Camera|PlayWorldCameraShake "/Game/Platformer/Blueprints/Blocks/PBlocks/BP_CameraShake.BP_CameraShake_C" (Transformation|GetActorLocation (Game|GetPlayerCharacter 0)) 1e+03 2e+03)
        (Game|Feedback|ClientPlayForceFeedback (Game|GetPlayerController 0) 0 "None" false false false))
      (:then_2
        ;[1 1 1] Show meshes and destroy components
        (Rendering|SetVisibility (Variables|Default|GetBlock_P_Top_Smashed) true false)
        (Components|DestroyComponent (Variables|Default|GetBox)))
      (:then_3
        ;[1 1 1] Find all actors with PBlock tag and turn ON function found in the Parent Block
        (bind _outactors (Actor|GetAllActorswithTag (Variables|Default|GetTag)))
        (bind _output_get (Variables|Default|SetBlocks _outactors))
        (for _array_element _output_get
          (bind _asbp_block_base (Utilities|Casting|CastToBP_Block_Base _array_element))
          (Default|PBlockon _asbp_block_base)))
      (:then_4
        ;[1 1 1] PBlock Timer
        (Utilities|Time|SetTimerbyEvent (delegate Custom|PBlockTimeOver) (Variables|Default|GetPBlockTimeDuration)))
      (:then_5
        (EventDispatchers|AssignPlayerStartsDeathSequence _asbp_third_person_character (delegate Custom|PlayerStartsDeathSequence_Event)))
      (:then_6
        (EventDispatchers|BindEventtoLevelComplete (Variables|Default|GetEndOfLevelFlag) (delegate Custom|LevelComplete_Event))))))

(event Custom|PBlockTimeOver
  ;[1 1 1] PBlock Timer
  (for _array_element (Variables|Default|GetBlocks)
    (bind _asbp_block_base (Utilities|Casting|CastToBP_Block_Base _array_element))
    (Utilities|IsValid _asbp_block_base
      (:Is%20Valid
        (Default|PBlockOff _asbp_block_base))
      (:Is%20Not%20Valid
        _))
    (Audio|Components|Audio|Stop (Variables|Default|GetMusic))
    ;[1 1 1] Unpause Level Music
    (Class|AudioComponent|SetPaused (Variables|/Game/Platformer/Blueprints/BP_LevelSettings.BP_LevelSettings_C|GetLevelMusic (Variables|Default|GetLevelSettings)) false)))

(event Custom|PlayerStartsDeathSequence_Event
  ;[1 1 1] PBlock Timer
  (for _array_element (Variables|Default|GetBlocks)
    (bind _asbp_block_base (Utilities|Casting|CastToBP_Block_Base _array_element))
    (Utilities|IsValid _asbp_block_base
      (:Is%20Valid
        (Default|PBlockOff _asbp_block_base))
      (:Is%20Not%20Valid
        _))
    (Audio|Components|Audio|Stop (Variables|Default|GetMusic))
    ;[1 1 1] Unpause Level Music
    (Class|AudioComponent|SetPaused (Variables|/Game/Platformer/Blueprints/BP_LevelSettings.BP_LevelSettings_C|GetLevelMusic (Variables|Default|GetLevelSettings)) false)))

(event Custom|LevelComplete_Event
  ;[1 1 1] PBlock Timer
  (for _array_element (Variables|Default|GetBlocks)
    (bind _asbp_block_base (Utilities|Casting|CastToBP_Block_Base _array_element))
    (Utilities|IsValid _asbp_block_base
      (:Is%20Valid
        (Default|PBlockOff _asbp_block_base))
      (:Is%20Not%20Valid
        _))
    (Audio|Components|Audio|Stop (Variables|Default|GetMusic))
    ;[1 1 1] Unpause Level Music
    (Class|AudioComponent|SetPaused (Variables|/Game/Platformer/Blueprints/BP_LevelSettings.BP_LevelSettings_C|GetLevelMusic (Variables|Default|GetLevelSettings)) false)))

(event EventBeginPlay)

(event Collision|EventActorBeginOverlap
  (params (OtherActor :type Actor%20Object%20Reference)))

(event EventTick
  (params (DeltaSeconds :type Float%20%28single-precision%29)))

(fn ConstructionScript)