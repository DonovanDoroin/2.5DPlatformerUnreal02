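; A question-mark coin block for a Mario-style platformer that pays out points and coins once when hit.
; The HitBlock event plays interact effects, swaps the cube material, spawns points and coin actors and credits both to the player controller.
; A timeline then bumps the cube along Z and a finished flag is set, so later hits only play a bump sound.
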(event EventBeginPlay
  (|CallParentFunction) ; This node is disabled and will not be called.\nDrag off pins to build functionality.
)

(event EventHitBlock
  (if (Variables|Default|GetIsFinishedInteracting)
    (Audio|PlaySound2D "/Game/Platformer/Audio/Mario_BrickBump.Mario_BrickBump" 1.0 1.0 0.0 0 0)
    (else
      (Utilities|FlowControl|Sequence
        (:then_0
          ;[1 1 1] Play FX
          (CallFunction|PlayBlockInteractEffect (Variables|Default|GetInteractSFX) (Variables|Default|GetInteractVFX%28Niagara%29) 0 (+ (Transformation|GetActorLocation) "0.000000,0.000000,50.000000"))
          (Rendering|Material|SetMaterial (Variables|Default|GetCube) 0 (Variables|Default|GetInteractMaterial)))
        (:then_1
          ;[1 1 1] Add Points
          (Game|SpawnActorfromClass "/Game/Platformer/Blueprints/BP_Points.BP_Points_C" (Transformation|GetActorTransform) "Undefined" "MultiplyWithRoot" 0 (Variables|Default|GetPoints) 0)
          (Default|AddPoints (Variables|Default|GetAsBPPlayerController) (Variables|Default|GetPoints)))
        (:then_2
          ;[1 1 1] Add Coins
          (Game|SpawnActorfromClass "/Game/Platformer/Blueprints/Blocks/BP_Block_Coin.BP_Block_Coin_C" (Transformation|GetActorTransform) "Undefined" "MultiplyWithRoot" 0 0)
          (Default|AddCoins (Variables|Default|GetAsBPPlayerController) (Variables|Default|GetCoinsToAdd)))
        (:then_3
          ;[1 1 1] Block Anim
          (bind _movement (Timeline|BlockAnim Play)
            (:Update
              (Transformation|SetRelativeLocation (Variables|Default|GetCube) (Math|Vector|MakeVector 0.0 0.0 _movement) false false))))
        (:then_4
          (Variables|Default|SetIsFinishedInteracting true))))))

(fn ConstructionScript
  (|CallParentFunction))