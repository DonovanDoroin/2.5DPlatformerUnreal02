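; Breakable brick block for a Mario-style platformer that reacts to being hit according to the player's hit points.
; If the player has at least two hit points, it plays interact effects, spawns a points actor, adds to the score via the player controller and destroys itself.
; Otherwise it plays a bump sound and bounces the cube vertically with a timeline.
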(event EventBeginPlay
  (|CallParentFunction) ; This node is disabled and will not be called.\nDrag off pins to build functionality.
)

(event EventHitBlock
  (bind _asbp_third_person_character (Utilities|Casting|CastToBP_ThirdPersonCharacter (Game|GetPlayerCharacter 0)))
  (if (>= (Variables|/Game/ThirdPerson/Blueprints/BP_ThirdPersonCharacter.BP_ThirdPersonCharacter_C|GetHitPoints _asbp_third_person_character) 2)
    (Utilities|FlowControl|Sequence
      (:then_0
        (CallFunction|PlayBlockInteractEffect (Variables|Default|GetInteractSFX) (Variables|Default|GetInteractVFX%28Niagara%29) 0 (Transformation|GetActorLocation)))
      (:then_1
        (Game|SpawnActorfromClass "/Game/Platformer/Blueprints/BP_Points.BP_Points_C" (Transformation|GetActorTransform) "Undefined" "MultiplyWithRoot" 0 (Variables|Default|GetPoints) 0)
        (Default|AddPoints (Variables|Default|GetAsBPPlayerController) (Variables|Default|GetPoints)))
      (:then_2
        (Actor|DestroyActor)))
    (else
      ;[1 1 1] Player small, don't break block
      (Audio|PlaySound2D "/Game/Platformer/Audio/Mario_BrickBump.Mario_BrickBump" 1.0 1.0 0.0 0 0)
      (bind _movement (Timeline|Timeline PlayFromStart)
        (:Update
          (Transformation|SetRelativeLocation (Variables|Default|GetCube) (Math|Vector|MakeVector 0.0 0.0 _movement) false false))))))

(fn ConstructionScript
  (|CallParentFunction))