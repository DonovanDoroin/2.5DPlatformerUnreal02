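; A coin actor, apparently for blocks, that plays a short animation as soon as it spawns and then removes itself.
; On BeginPlay the CoinAnim timeline runs at reduced speed, driving the coin's relative height and yaw.
; When the timeline finishes, it spawns a loot pickup particle effect at the coin's location and destroys the actor.
; It has no overlap or scoring logic.
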(event EventBeginPlay
  (bind _coin (Variables|Default|GetCoin))
  (bind _relativerotation (Variables|/Script/Engine.SceneComponent|GetRelativeRotation _coin))
  (Components|Timeline|SetPlayRate (Variables|Default|GetCoinAnim) 0.25)
  (bind (_direction _movement _rotation) (Timeline|CoinAnim PlayFromStart)
    (:Update
      (Transformation|SetRelativeLocationAndRotation (Variables|Default|GetCoin) (Math|Vector|MakeVectorNetQuantize 0.0 0.0 _movement) (Math|Rotator|MakeRotator (.roll _relativerotation) (.pitch _relativerotation) _rotation) false false))
    (:Finished
      (Effects|SpawnEmitteratLocation "/Game/InfinityBladeEffects/Effects/FX_Treasure/Loot/P_Loot_Pickup.P_Loot_Pickup" (Transformation|GetWorldLocation _coin))
      (Actor|DestroyActor))))

(event Collision|EventActorBeginOverlap
  (params (OtherActor :type Actor%20Object%20Reference)))

(event EventTick
  (params (DeltaSeconds :type Float%20%28single-precision%29)))

(fn ConstructionScript)