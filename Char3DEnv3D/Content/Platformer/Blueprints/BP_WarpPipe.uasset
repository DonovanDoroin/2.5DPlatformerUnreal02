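; Mario-style warp pipe that carries the player character from an entry point to a warp destination.
; An overlap gate lets up or down input, matching the pipe's direction, trigger entry when the pipe is interactable.
; Timelines slide the capsule in, then out rising or falling at the destination, with input disabled and warp sounds played.
; The construction script stacks instanced body segments downward according to the end point vector's length.
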(event OnComponentBeginOverlap(Collision)
  (params (OverlappedComponent :type Primitive%20Component%20Object%20Reference) (OtherActor :type Actor%20Object%20Reference) (OtherComp :type Primitive%20Component%20Object%20Reference) (OtherBodyIndex :type Integer) (bFromSweep :type Boolean) (SweepResult :type Hit%20Result%20Structure%20%28by%20ref%29))
  (bind _warpinpoint (Variables|Default|GetWarpInPoint))
  (bind _warptolocale (Variables|Default|GetWarpToLocale))
  (bind _warpinpoint_2 (Variables|Default|GetWarpInPoint))
  (bind _warptolocale_2 (Variables|Default|GetWarpToLocale))
  (bind _returnvalue (Transformation|GetWorldLocation _warpinpoint))
  (bind (_x _y _z) (Math|Vector|BreakVector _warptolocale))
  (bind _returnvalue_2 (Transformation|GetWorldLocation _warpinpoint_2))
  (bind (_x_2 _y_2 _z_2) (Math|Vector|BreakVector _warptolocale_2))
  (bind _asbp_third_person_character (Utilities|Casting|CastToBP_ThirdPersonCharacter OtherActor))
  (Utilities|FlowControl|Gate true) ; enters at Open
)

(event OnComponentEndOverlap(Collision)
  (params (OverlappedComponent :type Primitive%20Component%20Object%20Reference) (OtherActor :type Actor%20Object%20Reference) (OtherComp :type Primitive%20Component%20Object%20Reference) (OtherBodyIndex :type Integer))
  (bind _warpinpoint (Variables|Default|GetWarpInPoint))
  (bind _warptolocale (Variables|Default|GetWarpToLocale))
  (bind _warpinpoint_2 (Variables|Default|GetWarpInPoint))
  (bind _warptolocale_2 (Variables|Default|GetWarpToLocale))
  (bind _returnvalue (Transformation|GetWorldLocation _warpinpoint))
  (bind (_x _y _z) (Math|Vector|BreakVector _warptolocale))
  (bind _returnvalue_2 (Transformation|GetWorldLocation _warpinpoint_2))
  (bind (_x_2 _y_2 _z_2) (Math|Vector|BreakVector _warptolocale_2))
  (Utilities|Casting|CastToBP_ThirdPersonCharacter OtherActor)
  (Utilities|FlowControl|Gate true) ; enters at Close
)

(event Input|EnhancedActionEvents|EnhancedInputActionIA_PlayerUp
  (params (ActionValue :type Boolean) (ElapsedSeconds :type Float%20%28double-precision%29) (TriggeredSeconds :type Float%20%28double-precision%29) (InputAction :type Input%20Action%20Object%20Reference :default "/Game/ThirdPerson/Input/Actions/IA_PlayerUp.IA_PlayerUp"))
  (bind _warpinpoint (Variables|Default|GetWarpInPoint))
  (bind _warptolocale (Variables|Default|GetWarpToLocale))
  (bind _warpinpoint_2 (Variables|Default|GetWarpInPoint))
  (bind _warptolocale_2 (Variables|Default|GetWarpToLocale))
  (bind _returnvalue (Transformation|GetWorldLocation _warpinpoint))
  (bind (_x _y _z) (Math|Vector|BreakVector _warptolocale))
  (bind _returnvalue_2 (Transformation|GetWorldLocation _warpinpoint_2))
  (bind (_x_2 _y_2 _z_2) (Math|Vector|BreakVector _warptolocale_2))
  (if (and (Variables|Default|GetIsInteractable) (not (Variables|Default|GetIsDownPipe)))
    (Utilities|FlowControl|Gate true
      (:Exit
        (bind _output_get (Variables|Default|SetAs%20BP%20Third%20Person%20Character (stale OnComponentBeginOverlap(Collision) _asbp_third_person_character)))
        (Input|DisableInput _output_get (Game|GetPlayerController 0))
        (if (Variables|Default|GetIsDownPipe)
          (Utilities|FlowControl|Sequence
            (:then_0
              ;[1 1 1] Enter Down Pipe
              (bind _movement (Timeline|IntoDownPipe PlayFromStart)
                (:Update
                  (Transformation|SetRelativeLocationAndRotation (Variables|/Script/Engine.Character|GetCapsuleComponent (Variables|Default|GetAs%20BP%20Third%20Person%20Character)) (Math|Vector|MakeVector (.x _returnvalue_2) (.y _returnvalue_2) (+ (.z _returnvalue_2) _movement)) "0, 0, 0" false false))
                (:Finished
                  ;[1 1 1] Wait before exit out of pipe
                  (Utilities|FlowControl|Delay 0.4 :!label _label)
                  (Audio|PlaySound2D "/Game/Platformer/Audio/Mario_Warp.Mario_Warp" 1.0 1.0 0.0 0 0)
                  (if (Variables|Default|GetIsExitRisingUpOutOfPipe)
                    ;[1 1 1] Exit Rising Pipe
                    (bind _movement_2 (Timeline|Timeline PlayFromStart)
                      (:Update
                        (Transformation|SetRelativeLocationAndRotation (Variables|/Script/Engine.Character|GetCapsuleComponent (Variables|Default|GetAs%20BP%20Third%20Person%20Character)) (Math|Vector|MakeVector _x_2 _y_2 (+ _z_2 _movement_2)) "0, 0, 0" false false))
                      (:Finished
                        ;[1 1 1] Enabled User Control
                        (Input|EnableInput (Game|GetPlayerCharacter 0) (Game|GetPlayerController 0) :!label _label_2)))
                    (else
                      ;[1 1 1] Exit Falling Pipe
                      (bind _movement_3 (Timeline|Timeline_1 PlayFromStart)
                        (:Update
                          (Transformation|SetRelativeLocationAndRotation (Variables|/Script/Engine.Character|GetCapsuleComponent (Variables|Default|GetAs%20BP%20Third%20Person%20Character)) (Math|Vector|MakeVector _x _y (+ _z _movement_3)) "0, 0, 0" false false))
                        (:Finished
                          (goto _label_2))))))))
            (:then_1
              ;[1 1 1] Warp SFX
              (Utilities|FlowControl|Delay 0.2 :!label _label_3)
              (Audio|PlaySound2D "/Game/Platformer/Audio/Mario_Warp.Mario_Warp" 1.0 1.0 0.0 0 0)))
          (else
            (Utilities|FlowControl|Sequence
              (:then_0
                (goto _label_3))
              (:then_1
                ;[1 1 1] Enter Up Pipe
                (bind _movement_4 (Timeline|Timeline_0 PlayFromStart)
                  (:Update
                    (Transformation|SetRelativeLocationAndRotation (Variables|/Script/Engine.Character|GetCapsuleComponent (Variables|Default|GetAs%20BP%20Third%20Person%20Character)) (Math|Vector|MakeVector (.x _returnvalue) (.y _returnvalue) (+ (.z _returnvalue) _movement_4)) "0, 0, 0" false false))
                  (:Finished
                    (goto _label)))))))))))

(event Input|EnhancedActionEvents|EnhancedInputActionIA_PlayerDown
  (params (ActionValue :type Boolean) (ElapsedSeconds :type Float%20%28double-precision%29) (TriggeredSeconds :type Float%20%28double-precision%29) (InputAction :type Input%20Action%20Object%20Reference :default "/Game/ThirdPerson/Input/Actions/IA_PlayerDown.IA_PlayerDown"))
  (bind _warpinpoint (Variables|Default|GetWarpInPoint))
  (bind _warptolocale (Variables|Default|GetWarpToLocale))
  (bind _warpinpoint_2 (Variables|Default|GetWarpInPoint))
  (bind _warptolocale_2 (Variables|Default|GetWarpToLocale))
  (bind _returnvalue (Transformation|GetWorldLocation _warpinpoint))
  (bind (_x _y _z) (Math|Vector|BreakVector _warptolocale))
  (bind _returnvalue_2 (Transformation|GetWorldLocation _warpinpoint_2))
  (bind (_x_2 _y_2 _z_2) (Math|Vector|BreakVector _warptolocale_2))
  (if (and (Variables|Default|GetIsInteractable) (Variables|Default|GetIsDownPipe))
    (Utilities|FlowControl|Gate true
      (:Exit
        (bind _output_get (Variables|Default|SetAs%20BP%20Third%20Person%20Character (stale OnComponentBeginOverlap(Collision) _asbp_third_person_character)))
        (Input|DisableInput _output_get (Game|GetPlayerController 0))
        (if (Variables|Default|GetIsDownPipe)
          (Utilities|FlowControl|Sequence
            (:then_0
              ;[1 1 1] Enter Down Pipe
              (bind _movement (Timeline|IntoDownPipe PlayFromStart)
                (:Update
                  (Transformation|SetRelativeLocationAndRotation (Variables|/Script/Engine.Character|GetCapsuleComponent (Variables|Default|GetAs%20BP%20Third%20Person%20Character)) (Math|Vector|MakeVector (.x _returnvalue_2) (.y _returnvalue_2) (+ (.z _returnvalue_2) _movement)) "0, 0, 0" false false))
                (:Finished
                  ;[1 1 1] Wait before exit out of pipe
                  (Utilities|FlowControl|Delay 0.4 :!label _label)
                  (Audio|PlaySound2D "/Game/Platformer/Audio/Mario_Warp.Mario_Warp" 1.0 1.0 0.0 0 0)
                  (if (Variables|Default|GetIsExitRisingUpOutOfPipe)
                    ;[1 1 1] Exit Rising Pipe
                    (bind _movement_2 (Timeline|Timeline PlayFromStart)
                      (:Update
                        (Transformation|SetRelativeLocationAndRotation (Variables|/Script/Engine.Character|GetCapsuleComponent (Variables|Default|GetAs%20BP%20Third%20Person%20Character)) (Math|Vector|MakeVector _x_2 _y_2 (+ _z_2 _movement_2)) "0, 0, 0" false false))
                      (:Finished
                        ;[1 1 1] Enabled User Control
                        (Input|EnableInput (Game|GetPlayerCharacter 0) (Game|GetPlayerController 0) :!label _label_2)))
                    (else
                      ;[1 1 1] Exit Falling Pipe
                      (bind _movement_3 (Timeline|Timeline_1 PlayFromStart)
                        (:Update
                          (Transformation|SetRelativeLocationAndRotation (Variables|/Script/Engine.Character|GetCapsuleComponent (Variables|Default|GetAs%20BP%20Third%20Person%20Character)) (Math|Vector|MakeVector _x _y (+ _z _movement_3)) "0, 0, 0" false false))
                        (:Finished
                          (goto _label_2))))))))
            (:then_1
              ;[1 1 1] Warp SFX
              (Utilities|FlowControl|Delay 0.2 :!label _label_3)
              (Audio|PlaySound2D "/Game/Platformer/Audio/Mario_Warp.Mario_Warp" 1.0 1.0 0.0 0 0)))
          (else
            (Utilities|FlowControl|Sequence
              (:then_0
                (goto _label_3))
              (:then_1
                ;[1 1 1] Enter Up Pipe
                (bind _movement_4 (Timeline|Timeline_0 PlayFromStart)
                  (:Update
                    (Transformation|SetRelativeLocationAndRotation (Variables|/Script/Engine.Character|GetCapsuleComponent (Variables|Default|GetAs%20BP%20Third%20Person%20Character)) (Math|Vector|MakeVector (.x _returnvalue) (.y _returnvalue) (+ (.z _returnvalue) _movement_4)) "0, 0, 0" false false))
                  (:Finished
                    (goto _label)))))))))))

(event EventBeginPlay)

(event Collision|EventActorBeginOverlap
  (params (OtherActor :type Actor%20Object%20Reference)))

(event EventTick
  (params (DeltaSeconds :type Float%20%28single-precision%29)))

(fn ConstructionScript
  (for _index (range 0 (Math|Float|Truncate (/ (Math|Vector|VectorLength (Variables|Default|GetPipeEndPoint)) 1e+02)))
    (Components|InstancedStaticMesh|AddInstance (Variables|Default|GetPipeBody) (Math|Transform|MakeTransform (Math|Vector|MakeVector 0.0 0.0 (* _index -1e+02))) false)))