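; Per-level manager for a platformer that runs the countdown timer, level music and end-of-level transition.
; A looping timer decrements the HUD time on the player controller, plays a warning and raises music pitch when time is low, and kills the player at zero.
; Dispatchers from game mode, character and end flag reset on respawn, stop on death, or convert remaining time to points, save stats to the game instance and open the next level.
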(event Custom|PlayerRespawn
  (Utilities|FlowControl|Sequence
    (:then_0
      ;[1 1 1] Listen for "PlayerRespawn" Event Dispatcher in GameMode and reset level settings upon death
      (bind _asbp_third_person_game_mode (Utilities|Casting|CastToBP_ThirdPersonGameMode (Game|GetGameMode)))
      (EventDispatchers|AssignPlayerRespawn _asbp_third_person_game_mode (delegate Custom|PlayerRespawn_Event)))
    (:then_1
      ;[1 1 1] Ref to PlayerController and set Level Time Variable (Shown in HUD)
      (bind _asbp_player_controller (Utilities|Casting|CastToBP_PlayerController (Game|GetPlayerController 0)))
      (bind _output_get (Variables|Default|SetAs%20BP%20Player%20Controller _asbp_player_controller))
      (bind _output_get_2 (Variables|/Game/Platformer/Blueprints/Framework/BP_PlayerController.BP_PlayerController_C|SetLevelTime _output_get (Variables|Default|GetTimeLimitMax)))
      (Variables|Default|SetTimeLimitCurrent _output_get_2))
    (:then_2
      ;[1 1 1] Set audio to Populate our "LevelMusic"
      (Audio|Components|Audio|SetSound (Variables|Default|GetLevelMusic) (Variables|Default|GetLevelMusicVar))
      (Utilities|FlowControl|Delay 0.75)
      (Audio|Components|Audio|Play (Variables|Default|GetLevelMusic) 0.0))
    (:then_3
      ;[1 1 1] Run Timer and Play appropriate music depending on situation
      (Utilities|FlowControl|RetriggerableDelay 1.0)
      (bind _returnvalue (Utilities|Time|SetTimerbyEvent (delegate Custom|RunLevelTimer) (Variables|Default|GetTimePlayRate) true))
      (bind _output_get_3 (Variables|Default|SetLevelTimer _returnvalue)))
    (:then_4
      ;[1 1 1] Stop andy music when player dies. Event Dispatcher is called in 3rdPersonCharacterBP
      (bind _asbp_third_person_character (Utilities|Casting|CastToBP_ThirdPersonCharacter (Game|GetPlayerCharacter 0)))
      (EventDispatchers|BindEventtoPlayerStartsDeathSequence _asbp_third_person_character (delegate Custom|PlayerStartsDeathSequence_Event)))
    (:then_5
      (EventDispatchers|BindEventtoLevelComplete (Variables|Default|GetEndofLevelFlag) (delegate Custom|LevelComplete_Event)))))

(event Custom|PlayerRespawn_Event
  ;[1 1 1] Listen for "PlayerRespawn" Event Dispatcher in GameMode and reset level settings upon death
  (Audio|Components|Audio|SetPitchMultiplier (Variables|Default|GetLevelMusic) 1.0)
  (CallFunction|PlayerRespawn))

(event Custom|RunLevelTimer
  (bind _levelmusic (Variables|Default|GetLevelMusic))
  (bind _timelimitcurrent (Variables|Default|GetTimeLimitCurrent))
  ;[1 1 1] Run Timer and Play appropriate music depending on situation
  (if (== _timelimitcurrent 0)
    (Utilities|Time|ClearandInvalidateTimerbyHandle (stale Custom|PlayerRespawn _output_get_3))
    (Audio|Components|Audio|Stop (Variables|Default|GetTimeRunningOutWarning))
    (bind _asbp_third_person_character (Utilities|Casting|CastToBP_ThirdPersonCharacter (Game|GetPlayerCharacter 0)))
    (Default|PlayerDies _asbp_third_person_character)
    (else
      (bind _result (Math|Integer|DecrementInt _timelimitcurrent)
        (:%20%20
          (Variables|/Game/Platformer/Blueprints/Framework/BP_PlayerController.BP_PlayerController_C|SetLevelTime (Variables|Default|GetAs%20BP%20Player%20Controller) _result)
          (if (== _timelimitcurrent (Variables|Default|GetTimeRunningOutWarningVar))
            (Class|AudioComponent|SetPaused (Variables|Default|GetLevelMusic) true)
            (Audio|Components|Audio|Play (Variables|Default|GetTimeRunningOutWarning) 0.0)
            (Utilities|FlowControl|Delay 2.8)
            (Class|AudioComponent|SetPaused _levelmusic false)
            (Audio|Components|Audio|SetPitchMultiplier _levelmusic 1.05)))))))

(event Custom|PlayerStartsDeathSequence_Event
  ;[1 1 1] Stop andy music when player dies. Event Dispatcher is called in 3rdPersonCharacterBP
  (Audio|Components|Audio|Stop (Variables|Default|GetLevelMusic))
  (Utilities|Time|ClearandInvalidateTimerbyHandle (Variables|Default|GetLevelTimer)))

(event Custom|LevelComplete_Event
  (bind _returnvalue (Game|GetPlayerController 0))
  (bind _returnvalue_2 (Game|GetGameInstance))
  (bind _as_bp_player_controller (Variables|Default|GetAs%20BP%20Player%20Controller))
  (bind _asbp_player_controller (Utilities|Casting|CastToBP_PlayerController _returnvalue))
  (bind _asbp_game_instance (Utilities|Casting|CastToBP_GameInstance _returnvalue_2))
  (Audio|Components|Audio|Stop (Variables|Default|GetLevelMusic))
  (Utilities|Time|PauseTimerbyHandle (Variables|Default|GetLevelTimer))
  (Utilities|FlowControl|Delay 3.0)
  (Components|Activation|Activate (Variables|Default|GetLevelComplete) false)
  ;[1 1 1] Decrement time remaining when level is complete and award points
  (Utilities|FlowControl|Delay 0.05 :!label _label)
  (bind _result (Math|Integer|DecrementInt (Variables|/Game/Platformer/Blueprints/Framework/BP_PlayerController.BP_PlayerController_C|GetLevelTime _as_bp_player_controller))
    (:%20%20
      (if (> _result 0)
        (Default|AddPoints _as_bp_player_controller 50)
        (Audio|PlaySound2D "/Engine/VREditor/Sounds/UI/Camera_Shutter.Camera_Shutter" 1.0 1.0 0.0 0 0)
        (goto _label)
        (else
          (Variables|/Game/Platformer/Blueprints/Framework/BP_GameInstance.BP_GameInstance_C|SetCoins _asbp_game_instance (Variables|/Game/Platformer/Blueprints/Framework/BP_PlayerController.BP_PlayerController_C|GetCoins _asbp_player_controller))
          (Variables|/Game/Platformer/Blueprints/Framework/BP_GameInstance.BP_GameInstance_C|SetPoints _asbp_game_instance (Variables|/Game/Platformer/Blueprints/Framework/BP_PlayerController.BP_PlayerController_C|GetPoints _asbp_player_controller))
          (Variables|/Game/Platformer/Blueprints/Framework/BP_GameInstance.BP_GameInstance_C|SetLives _asbp_game_instance (Variables|/Game/Platformer/Blueprints/Framework/BP_PlayerController.BP_PlayerController_C|GetLives _asbp_player_controller))
          (Utilities|FlowControl|Delay 2.0)
          (Game|OpenLevel(byName) (Variables|Default|GetLevelToGoTo)))))))

(event EventBeginPlay
  (Utilities|FlowControl|Sequence
    (:then_0
      ;[1 1 1] Listen for "PlayerRespawn" Event Dispatcher in GameMode and reset level settings upon death
      (bind _asbp_third_person_game_mode (Utilities|Casting|CastToBP_ThirdPersonGameMode (Game|GetGameMode)))
      (EventDispatchers|AssignPlayerRespawn _asbp_third_person_game_mode (delegate Custom|PlayerRespawn_Event)))
    (:then_1
      ;[1 1 1] Ref to PlayerController and set Level Time Variable (Shown in HUD)
      (bind _asbp_player_controller (Utilities|Casting|CastToBP_PlayerController (Game|GetPlayerController 0)))
      (bind _output_get (Variables|Default|SetAs%20BP%20Player%20Controller _asbp_player_controller))
      (bind _output_get_2 (Variables|/Game/Platformer/Blueprints/Framework/BP_PlayerController.BP_PlayerController_C|SetLevelTime _output_get (Variables|Default|GetTimeLimitMax)))
      (Variables|Default|SetTimeLimitCurrent _output_get_2))
    (:then_2
      ;[1 1 1] Set audio to Populate our "LevelMusic"
      (Audio|Components|Audio|SetSound (Variables|Default|GetLevelMusic) (Variables|Default|GetLevelMusicVar))
      (Utilities|FlowControl|Delay 0.75)
      (Audio|Components|Audio|Play (Variables|Default|GetLevelMusic) 0.0))
    (:then_3
      ;[1 1 1] Run Timer and Play appropriate music depending on situation
      (Utilities|FlowControl|RetriggerableDelay 1.0)
      (bind _returnvalue (Utilities|Time|SetTimerbyEvent (delegate Custom|RunLevelTimer) (Variables|Default|GetTimePlayRate) true))
      (bind _output_get_3 (Variables|Default|SetLevelTimer _returnvalue)))
    (:then_4
      ;[1 1 1] Stop andy music when player dies. Event Dispatcher is called in 3rdPersonCharacterBP
      (bind _asbp_third_person_character (Utilities|Casting|CastToBP_ThirdPersonCharacter (Game|GetPlayerCharacter 0)))
      (EventDispatchers|BindEventtoPlayerStartsDeathSequence _asbp_third_person_character (delegate Custom|PlayerStartsDeathSequence_Event)))
    (:then_5
      (EventDispatchers|BindEventtoLevelComplete (Variables|Default|GetEndofLevelFlag) (delegate Custom|LevelComplete_Event)))))

(fn ConstructionScript)