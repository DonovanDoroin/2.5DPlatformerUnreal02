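; BP_Points is a short-lived actor that shows a points value popup in the platformer.
; On BeginPlay it casts its widget component's widget to W_Points, starts the PointsAnimation and writes PointsToAdd into the text block.
; It waits for the animation's end time, then destroys itself.
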(event EventBeginPlay
  (bind _asw_points (Utilities|Casting|CastToW_Points (UserInterface|GetWidget (Variables|Default|GetWidget))))
  (UserInterface|Animation|PlayAnimation _asw_points (Variables|/Game/Platformer/UI/W_Points.W_Points_C|GetPoints_Animation _asw_points) 0.0 1 "Forward" 1.0 false)
  (Variables|/Script/UMG.TextBlock|SetText (Variables|/Game/Platformer/UI/W_Points.W_Points_C|GetTextBlock_Points _asw_points) (Utilities|Text|ToText(Integer) (Variables|Default|GetPointsToAdd)))
  (Utilities|FlowControl|Delay (Class|WidgetAnimation|GetEndTime (Variables|/Game/Platformer/UI/W_Points.W_Points_C|GetPoints_Animation _asw_points)))
  (Actor|DestroyActor))

(fn ConstructionScript)