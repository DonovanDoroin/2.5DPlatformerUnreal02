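; Player controller for a Mario-style platformer that tracks coins, points and lives and owns the HUD and pause menu.
; BeginPlay adds the HUD widget; reaching 100 coins wraps the count, grants a life and plays a 1-up sound.
; Lives are clamped, and hitting zero opens the main menu level.
; The pause input toggles the pause menu and game pause, using mouse cursor visibility as the paused state.
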(event Custom|AddCoins
  (params (CoinsToAdd :type Integer))
  ;[1 1 1] AddCoins
  (if (>= (+ CoinsToAdd (Variables|Default|GetCoins)) 100)
    (Variables|Default|SetCoins (Math|Integer|Clamp(Integer) (- (+ CoinsToAdd (Variables|Default|GetCoins)) 100) 0 100))
    (CallFunction|AdjustLives 1)
    (Audio|PlaySound2D "/Game/Platformer/Audio/Mario_1up.Mario_1up" 1.0 1.0 0.0 0 0)
    (else
      (Variables|Default|SetCoins (Math|Integer|Clamp(Integer) (+ CoinsToAdd (Variables|Default|GetCoins)) 0 100)))))

(event Custom|AddPoints
  (params (PointsToAdd :type Integer))
  ;[1 1 1] Add Points
  (Variables|Default|SetPoints (+ PointsToAdd (Variables|Default|GetPoints))))

(event Custom|AdjustLives
  (params (LivesToAddOrSubtract :type Integer))
  ;[1 1 1] Adjust Lives
  (bind _output_get (Variables|Default|SetLives (Math|Integer|Clamp(Integer) (+ LivesToAddOrSubtract (Variables|Default|GetLives)) 0 99)))
  (if (== _output_get 0)
    (Game|OpenLevel(byName) "LV_MainMenu")))

(event Input|EnhancedActionEvents|EnhancedInputActionIA_Pause
  (params (ActionValue :type Boolean) (ElapsedSeconds :type Float%20%28double-precision%29) (TriggeredSeconds :type Float%20%28double-precision%29) (InputAction :type Input%20Action%20Object%20Reference :default "/Game/ThirdPerson/Input/Actions/IA_Pause.IA_Pause"))
  (:Started
    (if (Variables|Default|GetbShowMouseCursor)
      (Widget|RemovefromParent (Variables|Default|GetAs%20W%20Pause%20Menu))
      (Variables|Default|SetbShowMouseCursor false)
      (Audio|PlaySound2D "/Game/Platformer/Audio/Mario_Pause.Mario_Pause" 1.0 1.0 0.0 0 0)
      (Game|SetGamePaused false)
      (else
        (bind _returnvalue (UserInterface|CreateWidget "/Game/Platformer/UI/W_PauseMenu.W_PauseMenu_C"))
        (bind _output_get (Variables|Default|SetAs%20W%20Pause%20Menu _returnvalue))
        (UserInterface|Viewport|AddtoViewport _output_get 0)
        (Variables|Default|SetbShowMouseCursor true)
        (Audio|PlaySound2D "/Game/Platformer/Audio/Mario_Pause.Mario_Pause" 1.0 1.0 0.0 0 0)
        (Game|SetGamePaused true)))))

(event EventBeginPlay
  ;[1 1 1] Add HUD to Viewport
  (bind _returnvalue (UserInterface|CreateWidget "/Game/Platformer/UI/W_HUD.W_HUD_C"))
  (UserInterface|Viewport|AddtoViewport _returnvalue 0))

(fn ConstructionScript)